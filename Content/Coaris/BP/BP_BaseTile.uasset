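; BP_BaseTile is a self-destroying track tile, apparently the base for an endless-runner style level.
; When the third-person character overlaps its Box trigger, it asks the game mode to spawn another tile and adds a point scaled by the mode's multiplier.
; It also multiplies the player's walk speed by a speed-up factor, clamped between a fixed floor and MaxSpeed, then destroys itself after a short delay.
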(event `self.Box.OnComponentBeginOverlap`
  (params (OverlappedComponent :type "PrimitiveComponent Object Reference") (OtherActor :type "Actor Object Reference") (OtherComp :type "PrimitiveComponent Object Reference") (OtherBodyIndex :type Integer) (bFromSweep :type Boolean) (SweepResult :type "HitResult Structure (by ref)"))
  (cast `/Game/ThirdPerson/Blueprints/BP_ThirdPersonCharacter` OtherActor)
  ;[1 1 1] 生成新砖块
  (bind _asbp_third_person_game_mode (cast `/Game/ThirdPerson/Blueprints/BP_ThirdPersonGameMode` (`GameplayStatics.GetGameMode`)))
  (`/Game/ThirdPerson/Blueprints/BP_ThirdPersonGameMode.SpawnTile` _asbp_third_person_game_mode)
  ;[1 1 1] 增加得分
  (bind _asbp_third_person_game_mode_2 (cast `/Game/ThirdPerson/Blueprints/BP_ThirdPersonGameMode` (`GameplayStatics.GetGameMode`)))
  (set `/Game/ThirdPerson/Blueprints/BP_ThirdPersonGameMode.CurrentPoint` (+ (`/Game/ThirdPerson/Blueprints/BP_ThirdPersonGameMode.CurrentPoint` _asbp_third_person_game_mode_2) (* 1 (`/Game/ThirdPerson/Blueprints/BP_ThirdPersonGameMode.PointMultiplier` _asbp_third_person_game_mode_2))) _asbp_third_person_game_mode_2)
  (bind _asbp_third_person_character (cast `/Game/ThirdPerson/Blueprints/BP_ThirdPersonCharacter` (`GameplayStatics.GetPlayerCharacter` 0)))
  (bind _charactermovement (`Character.CharacterMovement` _asbp_third_person_character))
  (set `CharacterMovementComponent.MaxWalkSpeed` (`KismetMathLibrary.FClamp` (* (`CharacterMovementComponent.MaxWalkSpeed` _charactermovement) (`self.SpeedUpMultiplier`)) 600.0 (`self.MaxSpeed`)) _charactermovement)
  ;[1 1 1] 通过后销毁
  (`KismetSystemLibrary.Delay` 1.0)
  (`self.K2_DestroyActor`))

(fn `UserConstructionScript`)